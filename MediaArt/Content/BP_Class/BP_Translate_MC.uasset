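; BP_Translate_MC is an actor Blueprint that moves and rotates itself continuously every Tick, with Korean notes explaining the underlying P = Po + Vt math.
; Location advances along normalized DeltaLoc by Speed times delta time, without sweep.
; Rotation turns the actor's X axis by RotVect scaled by the same Speed and delta time, then rebuilds from that vector alone, so roll is not preserved.
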(event EventTick
  (params (DeltaSeconds :type Float%20%28single-precision%29))
  ;[0.15 0.15 0.15 0.5] 시간 = T
  ;[0.15 0.15 0.15 0.5] P = Po + Vt
  ; 변화될 위치 = 현재위치 + 방향x시간
  (Transformation|SetActorLocation (+ (Transformation|GetActorLocation) (* (* (Variables|Default|Getspeed) DeltaSeconds) (Math|Vector|Normalize (Variables|Default|GetdeltaLoc)))) false false)
  (Transformation|SetActorRotation (Math|Conversions|RotationFromXVector (Math|Vector|RotateVector (Math|Rotator|GetRotationXVector (Transformation|GetActorRotation)) (* (Variables|Default|GetrotVect) (* (Variables|Default|Getspeed) (Utilities|Time|GetWorldDeltaSeconds)))))))

(fn ConstructionScript)