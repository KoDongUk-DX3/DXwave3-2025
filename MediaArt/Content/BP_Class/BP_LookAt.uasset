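; BP_LookAt is an actor that turns to face the player pawn and chases it.
; BeginPlay and Tick share one chain that normalizes the vector to player 0's pawn and points the actor's X axis along it.
; The chain then moves the actor along that direction at a constant speed scaled by DeltaSeconds, without sweeping for collision.
; Disconnected leftover nodes include a character lookup and a reversed-facing rotation.
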(event EventBeginPlay
  ;[0.15 0.15 0.15 0.5] 방향구하는 노드
  ;;[0.15 0.15 0.15 0.5] 방향
  (bind _output_get (Variables|Default|Set방향 (Math|Vector|Normalize (- (Transformation|GetActorLocation (Game|Player|GetPlayerPawn 0)) (Transformation|GetActorLocation)))))
  (Transformation|SetActorRotation (Math|Rotator|MakeRotfromX _output_get))
  ;[0.15 0.15 0.15 0.5] 움직이는 노드
  ;;[0.15 0.15 0.15 0.5] P = Po + Vt
  ;; 변화될 위치 = 현재위치 + 방향x시간
  (Transformation|SetActorLocation (+ (Transformation|GetActorLocation) (* (* 1e+02 (stale EventTick DeltaSeconds)) (Variables|Default|Get방향))) false false))

(event EventTick
  (params (DeltaSeconds :type Float%20%28single-precision%29))
  ;[0.15 0.15 0.15 0.5] 움직이는 노드
  ;;[0.15 0.15 0.15 0.5] 시간 = T
  ;[0.15 0.15 0.15 0.5] 방향구하는 노드
  ;;[0.15 0.15 0.15 0.5] 방향
  (bind _output_get (Variables|Default|Set방향 (Math|Vector|Normalize (- (Transformation|GetActorLocation (Game|Player|GetPlayerPawn 0)) (Transformation|GetActorLocation)))))
  (Transformation|SetActorRotation (Math|Rotator|MakeRotfromX _output_get))
  ;;[0.15 0.15 0.15 0.5] P = Po + Vt
  ;; 변화될 위치 = 현재위치 + 방향x시간
  (Transformation|SetActorLocation (+ (Transformation|GetActorLocation) (* (* 1e+02 DeltaSeconds) (Variables|Default|Get방향))) false false))

(fn ConstructionScript)